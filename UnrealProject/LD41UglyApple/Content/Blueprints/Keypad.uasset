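; Keypad actor that opens the first FinalDoor when the correct code is entered while its externally controlled Allowed flag is set.
; Touchedkey appends the touched component's single-character name to Key, updates the display and compares against Solution once the length is reached.
; Success turns the pad green and locks input, while failure clears the entry and blinks the light through a DoN loop.
; A PlaySound helper stops the previous 2D cue before playing the next.
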(event `self.ReceiveBeginPlay`
  (bind _output_get (set `self.Key` ""))
  (set `self.Cleared` false)
  (set `self.Allowed` false)
  (`TextRenderComponent.K2_SetText` (`self.Display`) (`KismetTextLibrary.Conv_StringToText` _output_get))
  (bind _returnvalue (`GameplayStatics.CreateSound2D` "/Game/Audio/Input_Cue.Input_Cue"))
  (set `self.Sound` _returnvalue))

(event `Touched key`
  (params (Component :type "ActorComponent Object Reference"))
  (bind _returnvalue (`KismetSystemLibrary.GetObjectName` Component))
  (if (not (`self.Cleared`))
    (if (not (> (`KismetStringLibrary.Len` _returnvalue) 1))
      (bind _output_get (set `self.Key` (`KismetStringLibrary.Concat_StrStr` (`self.Key`) _returnvalue)))
      (`TextRenderComponent.K2_SetText` (`self.Display`) (`KismetTextLibrary.Conv_StringToText` _output_get))
      (if (>= (`KismetStringLibrary.Len` _output_get) (`KismetStringLibrary.Len` (`self.Solution`)))
        (if (and (== (`self.Key`) (`self.Solution`)) (`self.Allowed`))
          (set `self.Cleared` true)
          (`self.ChangeColor`)
          (`self.Play Sound` "/Game/Audio/Correct_Cue.Correct_Cue")
          (bind _outactors (`GameplayStatics.GetAllActorsOfClass` "/Game/Blueprints/FinalDoor.FinalDoor_C"))
          (`/Game/Blueprints/FinalDoor.Open Door` (`|GetArrayItem` _outactors))
          (else
            (set `self.Key` "")
            (`TextRenderComponent.K2_SetText` (`self.Display`) (`KismetTextLibrary.Conv_StringToText` ""))
            (`self.Play Sound` "/Game/Audio/Wrong_Cue.Wrong_Cue")
            (`self.BlinkColor`)))
        (else
          (`self.Play Sound` "/Game/Audio/Input_Cue.Input_Cue"))))))

(event `ChangeColor`
  (`PrimitiveComponent.SetMaterial` (`self.NumberPadBase`) 1 "/Game/Art/Props/NumberPad/numberpadGreen.numberpadGreen"))

(event `BlinkColor`
  (bind _counter (`/Engine/EditorBlueprintResources/StandardMacros.Do N` 3 :!label _label)
    (:`Exit`
      (`PrimitiveComponent.SetMaterial` (`self.NumberPadBase`) 1 "/Game/Art/Props/NumberPad/numberpadOff.numberpadOff")
      (`KismetSystemLibrary.Delay` 0.5)
      (`PrimitiveComponent.SetMaterial` (`self.NumberPadBase`) 1 "/Game/Art/Props/NumberPad/numberpadLight.numberpadLight")
      (`KismetSystemLibrary.Delay` 0.5)
      (if (< _counter 3)
        (goto _label)
        (else
          (goto _label :!via `Reset`))))))

(fn `Play Sound`
  (params (Sound :type "SoundCue Object Reference"))
  (bind _sound (`self.Sound`))
  (if (`AudioComponent.IsPlaying` _sound)
    (`AudioComponent.Stop` _sound))
  (bind _returnvalue (`GameplayStatics.SpawnSound2D` Sound))
  (set `self.Sound` _returnvalue))

(fn `UserConstructionScript`)