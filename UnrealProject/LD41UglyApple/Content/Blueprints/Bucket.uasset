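; Bucket is an interactable actor that supplies bait to the player and reports itself as not pickable.
; When used while open, it sets the player character's current bait to its own Bait value and shows that bait's name on the PlayerUI widget, found by a class search.
; Use always reports failure, even after changing the bait, and the currently equipped input is ignored.
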(fn `IsPickUp`
  (returns (IsPickup :type Boolean))
  (return false))

(fn `Use`
  (params (CurrentlyEquipped :type "Actor Object Reference"))
  (returns (Item :type "Actor Object Reference") (Success :type Boolean))
  (if (`self.Open`)
    (bind _ascharacter_base (cast `/Game/Blueprints/Character/Character_base` (`GameplayStatics.GetPlayerCharacter` 0)))
    (bind _output_get (set `/Game/Blueprints/Character/Character_base.CurrentBait` (`self.Bait`) _ascharacter_base))
    (bind _foundwidgets (`WidgetBlueprintLibrary.GetAllWidgetsOfClass` "/Game/Blueprints/Character/PlayerUI.PlayerUI_C"))
    (`/Game/Blueprints/Character/PlayerUI.SetBaitText` (`|GetArrayItem` _foundwidgets) (`|GetEnumeratorNameAsString` _output_get)))
  (return null false))

(fn `UserConstructionScript`)