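; A rotating door actor that swings open around its yaw axis when its TriggerDoor event is called.
; Shortly after BeginPlay it records its current yaw as the closed angle.
; TriggerDoor plays a timeline from the start, lerping relative yaw from the closed angle toward that angle plus MaxAngle, then sets IsOpen.
; There is no closing logic.
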(event `self.ReceiveBeginPlay`
  (bind (_returnvalue_roll _returnvalue_pitch _returnvalue_yaw) (`KismetMathLibrary.BreakRotator` (`self.K2_GetActorRotation`)))
  (`KismetSystemLibrary.Delay` 0.2)
  (set `self.DoorClosedAngle` _returnvalue_yaw))

(event `self.ReceiveActorBeginOverlap`
  (params (OtherActor :type "Actor Object Reference")))

(event `self.ReceiveTick`
  (params (DeltaSeconds :type "Float (single-precision)")))

(event `TriggerDoor`
  (bind _doorclosedangle (`self.DoorClosedAngle`))
  (bind (_direction _newtrack_0) (`Timeline|Timeline_0` :!via `PlayFromStart`)
    (:`Update`
      (`self.K2_SetActorRelativeRotation` (`KismetMathLibrary.MakeRotator` 0.0 0.0 (`KismetMathLibrary.Lerp` _doorclosedangle (+ _doorclosedangle (`self.MaxAngle`)) _newtrack_0))))
    (:`Finished`
      (set `self.IsOpen` true))))

(fn `UserConstructionScript`)