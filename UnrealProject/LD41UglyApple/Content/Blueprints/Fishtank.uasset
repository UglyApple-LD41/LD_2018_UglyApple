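; Fishtank actor that spawns wandering AI fish pawns with attached Eel actors inside its bounds and hosts a timed fishing minigame.
; Using a fishing rod stores the player's bait and starts a random wait, which Tick tracks to prompt a click.
; A second use inside the window spawns a bait-weighted or random catch, replacing the equipped item in front of the player.
; Using a held fish on the tank destroys it.
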(event EventBeginPlay
  (bind (_origin _boxextent) (Collision|GetActorBounds false))
  (for _index (range 0 5)
    (bind _returnvalue (AI|SpawnAIFromClass "/Game/Blueprints/AI/FishPawn.FishPawn_C" 0 (Math|Random|RandomPointinBoundingBox _origin _boxextent) (Math|Rotator|MakeRotator 0.0 0.0 (Math|Random|RandomFloatinRange 0.0 3.6e+02)) false))
    (bind _asfish_pawn (Utilities|Casting|CastToFishPawn _returnvalue))
    (Default|SetCurrentTank _asfish_pawn self)
    (bind _returnvalue_2 (Game|SpawnActorfromClass "/Game/Blueprints/Eel.Eel_C" (Transformation|GetActorTransform _returnvalue) "AlwaysSpawn" 0 0))
    (Transformation|AttachActorToActor _returnvalue_2 _returnvalue "None" "SnapToTarget" "SnapToTarget" "SnapToTarget" true)))

(event Collision|EventActorBeginOverlap
  (params (OtherActor :type Actor%20Object%20Reference)))

(event EventTick
  (params (DeltaSeconds :type Float%20%28single-precision%29))
  (bind _timebeforecatch (Variables|Default|GetTimeBeforeCatch))
  (if (Variables|Default|GetFishingMinigameOn)
    (bind _output_get (Variables|Default|SetCurrentTime (+ (Variables|Default|GetCurrentTime) DeltaSeconds)))
    (if (Math|Float|InRange(Float) _output_get _timebeforecatch (+ _timebeforecatch (Variables|Default|GetTimeToCatchFish)))
      (Development|PrintString "Click now!"))))

(fn ConstructionScript)

(fn CalculateFish
  (params (Bait :type Bait%20Enum :default "NewEnumerator0"))
  (switch Utilities|FlowControl|Switch|SwitchonBait Bait
    (:NewEnumerator0
      (bind _returnvalue (|SpawnEel))
      (CallFunction|SpawnFish _returnvalue))
    (:NewEnumerator1
      (bind _returnvalue_2 (|SpawnLobster))
      (CallFunction|SpawnFish _returnvalue_2)))
  (return))

(fn SpawnFish
  (params (PlayerRef :type Object%20Object%20Reference))
  (bind _returnvalue (Game|GetPlayerCharacter 0))
  (bind _fishtospawn (Variables|Default|GetFishToSpawn))
  (bind _ascharacter_base (Utilities|Casting|CastToCharacter_Base PlayerRef))
  (Transformation|DetachFromActor (Variables|/Game/Blueprints/Character/Character_base.Character_Base_C|GetCurrentlyEquipped _ascharacter_base) "KeepWorld" "KeepRelative" "KeepRelative")
  (Transformation|AttachActorToActor _fishtospawn (Game|GetPlayerCharacter 0) "None" "SnapToTarget" "KeepWorld" "KeepRelative" true)
  (bind _output_get (Variables|/Game/Blueprints/Character/Character_base.Character_Base_C|SetCurrentlyEquipped _ascharacter_base _fishtospawn))
  (Transformation|SetActorLocation _output_get (+ (Transformation|GetActorLocation _returnvalue) (* (Transformation|GetActorForwardVector _returnvalue) 100) (* (Transformation|GetActorRightVector _returnvalue) 25) (* (Transformation|GetActorUpVector (Variables|Default|GetFishToSpawn)) 25)) false false))

(fn IsPickUp
  (return false))

(fn Use
  (params (CurrentlyEquipped :type Actor%20Object%20Reference))
  (Utilities|Casting|CastToFishingRod CurrentlyEquipped
    (:then
      (if (Variables|Default|GetFishingMinigameOn)
        (if (Math|Float|InRange(Float) (Variables|Default|GetCurrentTime) (Variables|Default|GetTimeBeforeCatch) (+ (Variables|Default|GetTimeBeforeCatch) (Variables|Default|GetTimeToCatchFish)))
          (CallFunction|CalculateFish (Variables|Default|GetCurrentBait)))
        (Variables|Default|SetFishingMinigameOn false)
        (Variables|Default|SetCurrentTime 0.0)
        (else
          (bind _ascharacter_base (Utilities|Casting|CastToCharacter_Base (Game|GetPlayerCharacter 0)))
          (Variables|Default|SetCurrentBait (Variables|/Game/Blueprints/Character/Character_base.Character_Base_C|GetCurrentBait _ascharacter_base))
          (Variables|Default|SetFishingMinigameOn true)
          (Variables|Default|SetTimeBeforeCatch (Math|Random|RandomFloatinRange 2.0 15.0)))))
    (:CastFailed
      (bind _asfish (Utilities|Casting|CastToFish CurrentlyEquipped)
        (:then
          (Actor|DestroyActor _asfish))
        (:CastFailed
          _))))
  (return 0 (stale _bsuccess)))