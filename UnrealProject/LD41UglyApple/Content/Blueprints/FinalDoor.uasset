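; FinalDoor is a door actor that slides vertically open when its OpenDoor event is called.
; BeginPlay caches the starting Z position.
; OpenDoor waits briefly, plays a hydraulic sound in 2D, then runs the SlideUp timeline to lerp the actor's Z from that start by AmountToSlide, keeping X and Y unchanged.
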(event `self.ReceiveBeginPlay`
  (bind (_returnvalue_x _returnvalue_y _returnvalue_z) (`KismetMathLibrary.BreakVector` (`self.K2_GetActorLocation`)))
  (set `self.Starting Z` _returnvalue_z))

(event `Open Door`
  (bind (_returnvalue_x _returnvalue_y) (`KismetMathLibrary.BreakVector` (`self.K2_GetActorLocation`)))
  (`KismetSystemLibrary.Delay` 0.5)
  (`GameplayStatics.PlaySound2D` "/Game/Audio/FinalDoorHydraulic_Cue.FinalDoorHydraulic_Cue")
  (bind (_direction _alpha) (`Timeline|SlideUp`)
    (:`Update`
      (`self.K2_SetActorLocation` (`KismetMathLibrary.MakeVector` _returnvalue_x _returnvalue_y (`KismetMathLibrary.Lerp` (`self.Starting Z`) (+ (`self.Starting Z`) (`self.Amount to slide`)) _alpha))))))

(fn `UserConstructionScript`)