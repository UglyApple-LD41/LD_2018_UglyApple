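; BoxToOpen is an interactable, non-pickup actor that can hold a paper note.
; Its SpawnNote event spawns a PaperNote at the box's transform, assigns it the Note3 asset and stores the reference.
; Use sets Open on that note when HasNote is true, ignores the equipped item and always reports Success as false.
; Nothing in this Blueprint calls SpawnNote or sets HasNote.
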(event `SpawnNote`
  (bind _returnvalue (`|SpawnActorFromClass` "/Game/Blueprints/PaperNote.PaperNote_C" (`self.GetTransform`) "Undefined" "OverrideRootScale" null null))
  (set `/Game/Blueprints/PaperNote.NoteToShow` "/Game/Art/Props/SM_Notes_Note3.SM_Notes_Note3" _returnvalue)
  (set `self.NoteRef` _returnvalue))

(fn `IsPickUp`
  (returns (IsPickup :type Boolean))
  (return false))

(fn `Use`
  (params (CurrentlyEquipped :type "Actor Object Reference"))
  (returns (Item :type "Actor Object Reference") (Success :type Boolean))
  (if (`self.HasNote`)
    (set `/Game/Blueprints/PaperNote.Open` true (`self.NoteRef`)))
  (return null false))

(fn `UserConstructionScript`)