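; Exposed wires interactable that restores power when the player uses an Eel on it, and cannot be picked up.
; BeginPlay gives each BP_TL_Light a dynamic beam material and caches it.
; Use removes the particle effects, places the Eel on the wires and empties the player's hand.
; It then sets directional light and beam intensity, opens Buckets with a specific bait type and triggers the freezer door.
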(event `self.ReceiveBeginPlay`
  (bind _outactors (`GameplayStatics.GetAllActorsOfClass` "/Game/Blueprints/BP_TL_Light.BP_TL_Light_C"))
  (for _array_element _outactors
    (bind _returnvalue (`PrimitiveComponent.CreateDynamicMaterialInstance` (`StaticMeshActor.StaticMeshComponent` _array_element) 1 "/Game/Art/Environment/M_TLBeams_Inst.M_TLBeams_Inst"))
    (`KismetArrayLibrary.Array_Add` (`self.LightSources`) _returnvalue)))

(fn `IsPickUp`
  (returns (IsPickup :type Boolean))
  (return false))

(fn `Use`
  (params (CurrentlyEquipped :type "Actor Object Reference"))
  (returns (Item :type "Actor Object Reference") (Success :type Boolean))
  (bind (_aseel _bsuccess) (cast `/Game/Blueprints/Eel` CurrentlyEquipped :!pure true))
  (`ActorComponent.K2_DestroyComponent` (`self.ParticleSystem`))
  (`ActorComponent.K2_DestroyComponent` (`self.ParticleSystem1`))
  (`ActorComponent.K2_DestroyComponent` (`self.ParticleSystem2`))
  (`self.K2_DetachFromActor` _aseel "KeepRelative" "KeepRelative" "KeepRelative")
  (`self.K2_SetActorTransform` _aseel (`KismetMathLibrary.MakeTransform` (`self.K2_GetActorLocation`) (struct :`Pitch` 50.0 :`Roll` 115.0)) false false)
  (set `/Game/Blueprints/Character/Character_base.CurrentlyEquipped` (`self.EmptyActor`) (cast `/Game/Blueprints/Character/Character_base` (`GameplayStatics.GetPlayerCharacter` 0) :!pure true))
  (if _bsuccess
    (`LightComponent.SetIntensity` (`Light.LightComponent` (`self.DirectionalLight`)) 0.75)
    (for _array_element (`self.LightSources`)
      (`MaterialInstanceDynamic.SetScalarParameterValue` _array_element "Intensity" 2.0))
    (bind _outactors (`GameplayStatics.GetAllActorsOfClass` "/Game/Blueprints/Bucket.Bucket_C"))
    (for _array_element_2 _outactors
      (if (`|EnumEquality` (`/Game/Blueprints/Bucket.Bait` _array_element_2) "NewEnumerator1")
        (set `/Game/Blueprints/Bucket.Open` true _array_element_2)))
    (bind _outactors_2 (`GameplayStatics.GetAllActorsOfClass` "/Game/Blueprints/Freezer_door.Freezer_door_C"))
    (`/Game/Blueprints/Freezer_door.TriggerDoor` (`|GetArrayItem` _outactors_2)))
  (return null _bsuccess))

(fn `UserConstructionScript`)