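; PaperNote is a readable note actor that the player uses in place rather than picks up.
; Use disables player movement, spawns another PaperNote with the NoteToShow mesh, and attaches it in front of the character at a fixed relative transform.
; CloseNote restores walking and destroys the actor it is called on.
; BeginPlay stores the starting transform, which nothing here reads.
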(event `self.ReceiveBeginPlay`
  (set `self.StartTransform` (`self.GetTransform`)))

(event `CloseNote`
  (`CharacterMovementComponent.SetMovementMode` (`Character.CharacterMovement` (cast `/Game/Blueprints/Character/Character_base` (`GameplayStatics.GetPlayerCharacter` 0) :!pure true)) "MOVE_Walking" 0)
  (`self.K2_DestroyActor`))

(event `self.ReceiveTick`
  (params (DeltaSeconds :type "Float (single-precision)")))

(fn `IsPickUp`
  (returns (IsPickup :type Boolean))
  (return false))

(fn `Use`
  (params (CurrentlyEquipped :type "Actor Object Reference"))
  (returns (Item :type "Actor Object Reference") (Success :type Boolean))
  (bind _spawnednote (`self.SpawnedNote`))
  (`CharacterMovementComponent.DisableMovement` (`Character.CharacterMovement` (cast `/Game/Blueprints/Character/Character_base` (`GameplayStatics.GetPlayerCharacter` 0) :!pure true)))
  (bind _returnvalue (`|SpawnActorFromClass` "PaperNote_C" (`self.GetTransform`) "Undefined" "OverrideRootScale" null null))
  (set `self.SpawnedNote` _returnvalue)
  (`StaticMeshComponent.SetStaticMesh` (`StaticMeshActor.StaticMeshComponent` _returnvalue) (`self.NoteToShow`))
  (`self.K2_AttachToActor` _returnvalue (`GameplayStatics.GetPlayerCharacter` 0) "None" "KeepRelative" "KeepRelative" "KeepRelative" true)
  (`self.K2_SetActorRelativeLocation` _returnvalue (100.0 0.0 50.0) false false)
  (`self.K2_SetActorRelativeRotation` _spawnednote (struct :`Yaw` 180.0) false false)
  (`self.SetActorRelativeScale3D` _spawnednote (1.0 1.0 1.0))
  (return null true))

(fn `UserConstructionScript`)