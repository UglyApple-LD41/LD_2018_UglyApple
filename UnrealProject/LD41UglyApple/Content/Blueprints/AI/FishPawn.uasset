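; FishPawn is an AI fish pawn that tells its FishController which Fishtank it is in.
; On BeginPlay it takes the first overlapping Fishtank, and on later overlaps with a Fishtank it switches to that tank.
; Both paths call SetCurrentTank, which casts the pawn's controller to FishController and writes its CurrentTank variable.
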(event `self.ReceiveBeginPlay`
  (`self.SetCurrentTank` (cast `/Game/Blueprints/Fishtank` (`|GetArrayItem` (`self.GetOverlappingActors` "/Game/Blueprints/Fishtank.Fishtank_C")) :!pure true)))

(event `self.ReceiveActorBeginOverlap`
  (params (OtherActor :type "Actor Object Reference"))
  (bind _asfishtank (cast `/Game/Blueprints/Fishtank` OtherActor))
  (`self.SetCurrentTank` _asfishtank))

(fn `SetCurrentTank`
  (params (CurrentTank :type "/Game/Blueprints/Fishtank Object Reference"))
  (set `/Game/Blueprints/AI/FishController.CurrentTank` CurrentTank (cast `/Game/Blueprints/AI/FishController` (`self.GetController`) :!pure true)))

(fn `UserConstructionScript`)