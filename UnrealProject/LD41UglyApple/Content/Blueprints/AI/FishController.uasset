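; FishController is an AI controller that drives fish behavior through the FishBT behavior tree.
; On BeginPlay it starts the tree, then copies its wait timer, movement speed and turn speed variables into float blackboard keys, addressed through key-name variables.
; It has no active Tick or construction logic, leaving the behavior itself to the tree.
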(event `self.ReceiveBeginPlay`
  (bind _returnvalue (`AIBlueprintHelperLibrary.GetBlackboard` null))
  (`self.RunBehaviorTree` "/Game/Blueprints/AI/FishBT.FishBT")
  (`BlackboardComponent.SetValueAsFloat` _returnvalue (`self.WaitTimerName`) (`self.WaitTimer`))
  (`BlackboardComponent.SetValueAsFloat` _returnvalue (`self.MovementSpeedName`) (`self.MovementSpeed`))
  (`BlackboardComponent.SetValueAsFloat` _returnvalue (`self.TurnSpeedName`) (`self.TurnSpeed`)))

(fn `UserConstructionScript`)