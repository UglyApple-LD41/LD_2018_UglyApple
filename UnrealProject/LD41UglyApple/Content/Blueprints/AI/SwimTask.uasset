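; Behavior tree task that swims a FishPawn toward the NextPos blackboard location.
; Each tick it moves and turns the pawn by constant-rate interpolation, using MovementSpeed and TurnSpeed from the blackboard.
; It passes FishPawn.Swim a state based on whether the fish is turning, which way, or finished.
; The task succeeds within Delta of the target and fails if setting location and rotation returns false.
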(event `self.ReceiveTickAI`
  (params (OwnerController :type "AIController Object Reference") (ControlledPawn :type "Pawn Object Reference") (DeltaSeconds :type "Float (single-precision)"))
  (bind _returnvalue (`Actor.K2_GetActorLocation` ControlledPawn))
  (bind _returnvalue_2 (`Actor.K2_GetActorRotation` ControlledPawn))
  (bind _asfish_pawn (cast `/Game/Blueprints/AI/FishPawn` ControlledPawn :!pure true))
  (bind _returnvalue_3 (`BTFunctionLibrary.GetBlackboardValueAsVector` (`self.NextPos`)))
  (bind _returnvalue_4 (`KismetMathLibrary.FindLookAtRotation` _returnvalue _returnvalue_3))
  (set `self.Dir` (> (`KismetMathLibrary.ClampAxis` (- (.yaw _returnvalue_4) (.yaw _returnvalue_2))) 180.0))
  (set `self.Rotating` (not (== _returnvalue_4 _returnvalue_2 :`ErrorTolerance` 2.0)))
  (bind (_sweephitresult _returnvalue_5) (`Actor.K2_SetActorLocationAndRotation` ControlledPawn (`KismetMathLibrary.VInterpTo_Constant` _returnvalue _returnvalue_3 DeltaSeconds (`BTFunctionLibrary.GetBlackboardValueAsFloat` (`self.MovementSpeed`))) (`KismetMathLibrary.RInterpTo_Constant` _returnvalue_2 _returnvalue_4 DeltaSeconds (`BTFunctionLibrary.GetBlackboardValueAsFloat` (`self.TurnSpeed`))) false false))
  (if _returnvalue_5
    (if (== (`BTFunctionLibrary.GetBlackboardValueAsVector` (`self.NextPos`)) (`Actor.K2_GetActorLocation` ControlledPawn) :`ErrorTolerance` (`self.Delta`))
      (`/Game/Blueprints/AI/FishPawn.Swim` _asfish_pawn "NewEnumerator3")
      (`self.FinishExecute` true)
      (elif (`self.Rotating`)
        (if (`self.Dir`)
          (`/Game/Blueprints/AI/FishPawn.Swim` _asfish_pawn "NewEnumerator1")
          (else
            (`/Game/Blueprints/AI/FishPawn.Swim` _asfish_pawn "NewEnumerator2")))
        (else
          (`/Game/Blueprints/AI/FishPawn.Swim` _asfish_pawn "NewEnumerator0"))))
    (else
      (`/Game/Blueprints/AI/FishPawn.Swim` _asfish_pawn "NewEnumerator3")
      (`self.FinishExecute` false))))